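; FallingWall_BP is a wall that lowers out of the way when its item-deposit open request fires, then destroys itself.
; A timeline subtracts its Height track from the actor's Z, using a location sampled by a Get Location event track through a helper function.
; Other event tracks start and stop the wall-moving sound in sync with the motion.
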(event `self.Entr_ItemDeposited.OpenRequest`
  (bind _wallmoving (`self.WallMoving`))
  (bind (_direction _height) (`Timeline|Timeline_0`)
    (:`Update`
      (`self.K2_SetActorLocation` (`KismetMathLibrary.MakeVector` (stale _returnvalue_x) (stale _returnvalue_y) (- (stale _returnvalue_z) _height))))
    (:`Finished`
      (`self.K2_DestroyActor`))
    (:`GetLocation`
      (bind (_returnvalue_x _returnvalue_y _returnvalue_z) (`self.NewFunction_0`)))
    (:`PlayAudio`
      (`AudioComponent.Play` _wallmoving 0.0)
      (`self.K2_SetActorLocation` (`self.K2_GetActorLocation`)))
    (:`StopAudio`
      (`AudioComponent.Stop` _wallmoving))))

(fn `NewFunction_0`
  (returns (ReturnValue_X :type "Float (double-precision)") (ReturnValue_Y :type "Float (double-precision)") (ReturnValue_Z :type "Float (double-precision)"))
  (bind (_returnvalue_x _returnvalue_y _returnvalue_z) (`KismetMathLibrary.BreakVector` (`self.K2_GetActorLocation`)))
  (return _returnvalue_x _returnvalue_y _returnvalue_z))

(fn `UserConstructionScript`)