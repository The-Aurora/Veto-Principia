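; Falling wall actor that alternates its location between a start height and an underground height on a repeating cycle.
; BeginPlay caches coordinates through NewFunction1, which returns actor Z as X and zeros for Y and Z, leaving NewFunction0 unused.
; Two chained timelines, each given a random 0–5 value, loop.
; Their updates set fixed offset positions without interpolation, the second supplying only Z.
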(event `self.ReceiveBeginPlay`
  (`|ExecutionSequence`
    (:`then_0`
      (bind (_returnvalue_x _returnvalue_y _returnvalue_z) (`self.NewFunction_1`))
      (`|ExecutionSequence`
        (:`then_0`
          (set `self.ActorXLocation` _returnvalue_x))
        (:`then_1`
          (set `self.ActorYLocation` _returnvalue_y))
        (:`then_2`
          (bind _output_get (set `self.ActorZLocationStart` _returnvalue_z))
          (set `self.ActorZLocationEnd` (- _output_get (`self.ZValueToGoUnderGround`))))))
    (:`then_1`
      (`Timeline|Timeline_0` :`NewTime` (`KismetMathLibrary.RandomFloatInRange` 0.0 5.0) :!label _label
        (:`Update`
          (`self.K2_SetActorLocation` (`KismetMathLibrary.MakeVector` (`self.ActorXLocation`) (`self.ActorYLocation`) (- (`self.ActorZLocationStart`) 1.0))))
        (:`Finished`
          (`Timeline|Timeline_1` :`NewTime` (`KismetMathLibrary.RandomFloatInRange` 0.0 5.0)
            (:`Update`
              (`self.K2_SetActorLocation` (`KismetMathLibrary.MakeVector` 0.0 0.0 (+ (`self.ActorZLocationEnd`) 1.0))))
            (:`Finished`
              (goto _label :!via `PlayFromStart`))))))))

(fn `NewFunction_0`
  (returns (ReturnValue_X :type "Float (double-precision)") (ReturnValue_Y :type "Float (double-precision)") (ReturnValue_Z :type "Float (double-precision)"))
  (bind (_returnvalue_x _returnvalue_y _returnvalue_z) (`KismetMathLibrary.BreakVector` (`self.K2_GetActorLocation`)))
  (return _returnvalue_x _returnvalue_y _returnvalue_z))

(fn `NewFunction_1`
  (returns (ReturnValue_X :type "Float (double-precision)") (ReturnValue_Y :type "Float (double-precision)") (ReturnValue_Z :type "Float (double-precision)"))
  (bind (_returnvalue_x _returnvalue_y _returnvalue_z) (`KismetMathLibrary.BreakVector` (`self.K2_GetActorLocation`)))
  (return _returnvalue_z 0.0 0.0))

(fn `UserConstructionScript`)