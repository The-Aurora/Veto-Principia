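; Moving platform actor for Segment 3 that rises and then slides sideways when the S3_GoalReached ElevatePlatform event fires.
; A first timeline adds its Height curve to Z, and on finishing starts a second timeline that subtracts its Horizontal curve from Y.
; Each timeline's Get Actor Location event track captures the current position through a helper function as the base for that movement's offset.
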(event `self.S3_GoalReached.ElevatePlatform`
  (bind (_direction _height) (`Timeline|Timeline_0`)
    (:`Update`
      (`self.K2_SetActorLocation` (`KismetMathLibrary.MakeVector` (stale _returnvalue_x_2) (stale _returnvalue_y_2) (+ (stale _returnvalue_z_2) _height))))
    (:`Finished`
      (bind (_direction_2 _horizontal) (`Timeline|Timeline_1`)
        (:`Update`
          (`self.K2_SetActorLocation` (`KismetMathLibrary.MakeVector` (stale _returnvalue_x) (- (stale _returnvalue_y) _horizontal) (stale _returnvalue_z))))
        (:`GetActorLocation`
          (bind (_returnvalue_x _returnvalue_y _returnvalue_z) (`self.NewFunction_1`)))))
    (:`GetActorLocation`
      (bind (_returnvalue_x_2 _returnvalue_y_2 _returnvalue_z_2) (`self.NewFunction_0`)))))

(fn `NewFunction_0`
  (returns (ReturnValue_X :type "Float (double-precision)") (ReturnValue_Y :type "Float (double-precision)") (ReturnValue_Z :type "Float (double-precision)"))
  (bind (_returnvalue_x _returnvalue_y _returnvalue_z) (`KismetMathLibrary.BreakVector` (`self.K2_GetActorLocation`)))
  (return _returnvalue_x _returnvalue_y _returnvalue_z))

(fn `NewFunction_1`
  (returns (ReturnValue_X :type "Float (double-precision)") (ReturnValue_Y :type "Float (double-precision)") (ReturnValue_Z :type "Float (double-precision)"))
  (bind (_returnvalue_x _returnvalue_y _returnvalue_z) (`KismetMathLibrary.BreakVector` (`self.K2_GetActorLocation`)))
  (return _returnvalue_x _returnvalue_y _returnvalue_z))

(fn `UserConstructionScript`)