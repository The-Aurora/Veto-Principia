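; Moving platform Blueprint that shifts its actor in four directions, one per position event from its C++ CirclePlatform logic.
; Each event plays its own timeline from the start, moving along +X, -Y, -X or +Y for positions one to four.
; On each update it reads the current location through C++ getters and adds or subtracts the timeline value on one axis, so offsets accumulate.
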(event `self.CirclePlatform.PositionOne`
  (bind _circleplatform (`self.CirclePlatform`))
  ;[1 1 1] Positions to change location based on (see C++ for deterministic logic)
  ;;[1 1 1] Position One
  (bind (_direction _value) (`Timeline|Timeline_0` :!via `PlayFromStart`)
    (:`Update`
      (`|ExecutionSequence`
        (:`then_0`
          (bind _returnvalue (`CirclePlatform.GetLocationX` _circleplatform)))
        (:`then_1`
          (bind _returnvalue_2 (`CirclePlatform.GetLocationY` _circleplatform)))
        (:`then_2`
          (bind _returnvalue_3 (`CirclePlatform.GetLocationZ` _circleplatform)))
        (:`then_3`
          (`self.K2_SetActorLocation` (`KismetMathLibrary.MakeVector` (+ _returnvalue _value) _returnvalue_2 _returnvalue_3)))))))

(event `self.CirclePlatform.PositionThree`
  (bind _circleplatform (`self.CirclePlatform`))
  ;[1 1 1] Positions to change location based on (see C++ for deterministic logic)
  ;;[1 1 1] Position Two
  (bind (_direction _value) (`Timeline|Timeline_2` :!via `PlayFromStart`)
    (:`Update`
      (`|ExecutionSequence`
        (:`then_0`
          (bind _returnvalue (`CirclePlatform.GetLocationX` _circleplatform)))
        (:`then_1`
          (bind _returnvalue_2 (`CirclePlatform.GetLocationY` _circleplatform)))
        (:`then_2`
          (bind _returnvalue_3 (`CirclePlatform.GetLocationZ` _circleplatform)))
        (:`then_3`
          (`self.K2_SetActorLocation` (`KismetMathLibrary.MakeVector` (- _returnvalue _value) _returnvalue_2 _returnvalue_3)))))))

(event `self.CirclePlatform.PositionTwo`
  (bind _circleplatform (`self.CirclePlatform`))
  ;[1 1 1] Positions to change location based on (see C++ for deterministic logic)
  ;;[1 1 1] Position Two
  (bind (_direction _value) (`Timeline|Timeline_1` :!via `PlayFromStart`)
    (:`Update`
      (`|ExecutionSequence`
        (:`then_0`
          (bind _returnvalue (`CirclePlatform.GetLocationX` _circleplatform)))
        (:`then_1`
          (bind _returnvalue_2 (`CirclePlatform.GetLocationY` _circleplatform)))
        (:`then_2`
          (bind _returnvalue_3 (`CirclePlatform.GetLocationZ` _circleplatform)))
        (:`then_3`
          (`self.K2_SetActorLocation` (`KismetMathLibrary.MakeVector` _returnvalue (- _returnvalue_2 _value) _returnvalue_3)))))))

(event `self.CirclePlatform.PositionFour`
  (bind _circleplatform (`self.CirclePlatform`))
  ;[1 1 1] Positions to change location based on (see C++ for deterministic logic)
  ;;[1 1 1] Position Two
  (bind (_direction _value) (`Timeline|Timeline_3` :!via `PlayFromStart`)
    (:`Update`
      (`|ExecutionSequence`
        (:`then_0`
          (bind _returnvalue (`CirclePlatform.GetLocationX` _circleplatform)))
        (:`then_1`
          (bind _returnvalue_2 (`CirclePlatform.GetLocationY` _circleplatform)))
        (:`then_2`
          (bind _returnvalue_3 (`CirclePlatform.GetLocationZ` _circleplatform)))
        (:`then_3`
          (`self.K2_SetActorLocation` (`KismetMathLibrary.MakeVector` _returnvalue (+ _returnvalue_2 _value) _returnvalue_3)))))))

(fn `UserConstructionScript`)